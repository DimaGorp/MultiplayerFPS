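; BP_GameMode is a game mode Blueprint that provides player respawning through a RespawnPlayer event taking a Controller.
; If the controller has a valid pawn, the event destroys it and spawns a new BP_Player at a randomly chosen PlayerStart.
; The spawn adjusts for collisions but always succeeds, and the controller then possesses the new pawn.
; A controller without a valid pawn is not respawned.
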(event `RespawnPlayer`
  (params (Controller :type "Controller Object Reference"))
  (bind _returnvalue (`Controller.K2_GetPawn` Controller))
  (bind _outactors (`GameplayStatics.GetAllActorsOfClass` "/Script/Engine.PlayerStart"))
  (`/Engine/EditorBlueprintResources/StandardMacros.IsValid` _returnvalue
    (:`Is Valid`
      (`self.K2_DestroyActor` _returnvalue)
      (bind _returnvalue_2 (`|SpawnActorFromClass` "/Game/Bluprints/Player/BP_Player.BP_Player_C" (`self.GetTransform` (`|GetArrayItem` _outactors (`KismetMathLibrary.RandomIntegerInRange` 0 (- (`KismetArrayLibrary.Array_Length` _outactors) 1)))) "AdjustIfPossibleButAlwaysSpawn" "MultiplyWithRoot" null null))
      (`Controller.Possess` Controller _returnvalue_2))))

(fn `UserConstructionScript`)