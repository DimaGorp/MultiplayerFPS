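; BP_Knife is a knife weapon Blueprint that customizes the Fire function inherited from its parent.
; Its Fire override discards the caller's start and end locations, substituting the world positions of two Arrow components on the knife.
; It adds itself to the ignored actors, then delegates to the parent Fire and returns that result.
; The event graph is empty, and construction only calls the parent script.
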(fn `Fire`
  (params (StartLocation :type "Vector Structure") (EndLocation :type "Vector Structure") (IgnoreActors :type "Array of Actor Object Reference (by ref)") (`Debug?` :type Boolean))
  (returns (`Hit Result Structure` :type "HitResult Structure"))
  (`KismetArrayLibrary.Array_Append` IgnoreActors (`|MakeArray` self :!type "Actor Object Reference"))
  (bind _hit_result_structure (`parent.Fire` (`SceneComponent.K2_GetComponentLocation` (`self.Arrow`)) (`SceneComponent.K2_GetComponentLocation` (`self.Arrow1`)) IgnoreActors `Debug?`))
  (return _hit_result_structure))

(fn `UserConstructionScript`
  (`parent.UserConstructionScript`))