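; BP_Pistol_1991 is a pistol weapon Blueprint that builds on a parent weapon class.
; It overrides Fire to add itself to the ignored actors and pass the parent a 1000-unit trace along its Arrow component, replacing the caller's start and end points.
; An interact event destroys the actor, and DecreaseAmmo lowers Ammo by one while it is above zero.
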(event `Itteract_1`
  (`self.K2_DestroyActor`))

(event `/Game/Bluprints/BP_Interface/BP_IReloader.DecreaseAmmo`
  (if (> (`self.Ammo`) 0)
    (`/Engine/EditorBlueprintResources/StandardMacros.DecrementInt` (`self.Ammo`))))

(fn `Fire`
  (params (StartLocation :type "Vector Structure") (EndLocation :type "Vector Structure") (IgnoreActors :type "Array of Actor Object Reference (by ref)") (`Debug?` :type Boolean))
  (returns (`Hit Result Structure` :type "HitResult Structure"))
  (bind _arrow (`self.Arrow`))
  (bind _returnvalue (`SceneComponent.K2_GetComponentLocation` _arrow))
  (`KismetArrayLibrary.Array_Append` IgnoreActors (`|MakeArray` self :!type "Actor Object Reference"))
  (bind _hit_result_structure (`parent.Fire` _returnvalue (+ _returnvalue (* (`SceneComponent.GetForwardVector` _arrow) 1000.0)) IgnoreActors `Debug?`))
  (return _hit_result_structure))

(fn `UserConstructionScript`
  (`parent.UserConstructionScript`))