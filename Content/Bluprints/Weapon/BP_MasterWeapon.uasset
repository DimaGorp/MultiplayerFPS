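; BP_MasterWeapon is a weapon Blueprint, named as the master weapon, that provides hitscan firing.
; Its Fire function checks that Ammo is above zero, then line traces on the Visibility channel between given points, with ignored actors and optional debug drawing.
; It returns the hit result on a hit, without reducing Ammo or applying damage.
; The event graph holds only an empty cursor-over event and unconnected trace nodes.
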(event `self.ReceiveActorBeginCursorOver`)

(fn `Fire`
  (params (StartLocation :type "Vector Structure") (EndLocation :type "Vector Structure") (IgnoreActors :type "Array of Actor Object Reference (by ref)") (`Debug?` :type Boolean))
  (returns (`Hit Result Structure` :type "HitResult Structure"))
  (if (> (`self.Ammo`) 0)
    (bind (_outhit _returnvalue) (`KismetSystemLibrary.LineTraceSingle` StartLocation EndLocation "TraceTypeQuery1" false IgnoreActors (select `bool` `Debug?` :`true` "ForDuration" :!type "EDrawDebugTrace Enum")))
    (if _returnvalue
      (return _outhit))))

(fn `UserConstructionScript`)