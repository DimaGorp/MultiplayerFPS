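; BPC_Inventory is an inventory component that adds items to an Inventory array by item ID.
; AddItemToInventory looks up the ID as a row name in InventoryDataTable and appends the found row.
; An empty inventory takes the item directly; otherwise an empty loop runs first, so only the last element's WeaponName is compared to block a duplicate.
; BeginPlay and Tick do nothing.
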(event `self.ReceiveBeginPlay`)

(fn `AddItemToInventory`
  (params (ItemID :type "Name (by ref)"))
  (if (`KismetArrayLibrary.Array_IsEmpty` (`self.inventory`))
    (bind _returnvalue (`|GetDataTableRow` "/Game/Bluprints/Data/InventoryDataTable.InventoryDataTable" ItemID :!label _label)
      (:`then`
        (`KismetArrayLibrary.Array_Add` (`self.inventory`) _returnvalue)))
    (else
      (for _array_element (`self.inventory`)
        _)
      (if (!= (`.WeaponName_10_DCE549F14E77AFB4B2CE7DA4692A0AC9` (break `/Game/Bluprints/Data/S_ItemData` _array_element)) ItemID)
        (goto _label)))))